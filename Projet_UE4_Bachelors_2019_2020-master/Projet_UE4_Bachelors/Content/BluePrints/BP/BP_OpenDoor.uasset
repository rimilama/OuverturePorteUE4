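; BP_OpenDoor is a door that opens when enough mass rests on a linked pressure plate actor, Plaque.
; Each begin or end overlap on the plate resets PoidsTotal, then SetPoidsTotal sums the static mesh masses of all actors overlapping it.
; Tick plays or reverses the Ouverture_porte timeline against a weight threshold, with the timeline driving the door's yaw and a Sound event playing the lock sound.
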(event OnActorBeginOverlap(Plaque)
  (params (OverlappedActor :type Actor%20Object%20Reference) (OtherActor :type Actor%20Object%20Reference))
  ;[1 1 1] Mise a jour du poids total lors de l'entrée ou de la sortie d'un objet
  (Variables|Default|SetPoids%20total 0.0)
  (CallFunction|SetPoidsTotal OverlappedActor))

(event OnActorEndOverlap(Plaque)
  (params (OverlappedActor :type Actor%20Object%20Reference) (OtherActor :type Actor%20Object%20Reference))
  ;[1 1 1] Mise a jour du poids total lors de l'entrée ou de la sortie d'un objet
  (Variables|Default|SetPoids%20total 0.0)
  (CallFunction|SetPoidsTotal OverlappedActor))

(event EventTick
  (params (DeltaSeconds :type Float%20%28single-precision%29))
  ;[1 1 1] Lancement animation selon le poids total
  (if (>= (Variables|Default|GetPoids%20total) 1.1e+02)
    (bind _ouverture (Timeline|Ouverture_porte Play)
      (:Update
        (Transformation|SetActorRotation (Math|Rotator|MakeRotator 0.0 0.0 _ouverture)))
      (:Sound
        (Audio|PlaySoundatLocation "/Game/Sound/door-lock.door-lock" (Transformation|GetActorLocation) "0, 0, 0" 1.0 1.0 0.0 0 0 0)))
    (else
      (Timeline|Ouverture_porte Reverse))))

(fn ConstructionScript)

(fn SetPoidsTotal
  (params (ObjetCourrant :type Actor%20Object%20Reference))
  (bind _output_get (Variables|Default|SetTableauObjet (Collision|GetOverlappingActors ObjetCourrant "/Script/Engine.Actor" :!class /Script/Engine.Actor)))
  (for _array_element _output_get
    (Variables|Default|SetPoids%20total (+ (Variables|Default|GetPoids%20total) (Physics|GetMass (Actor|GetComponentbyClass _array_element "/Script/Engine.StaticMeshComponent"))))))